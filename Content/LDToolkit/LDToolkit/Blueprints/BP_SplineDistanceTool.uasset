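; Editor spline measuring tool that displays the spline's length as text and lines the spline with copies of a chosen static mesh.
; The construction script derives the spacing from the mesh's bounding-box X size times a size multiplier.
; It rebuilds instanced static mesh copies at that interval along the spline, uniformly scaled but not rotated to follow it, then applies the main color material.
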(fn `UserConstructionScript`
  (bind _static_mesh_size_multiplier (`self.Static Mesh Size Multiplier`))
  (bind (_returnvalue_min _returnvalue_max) (break `Box` (`StaticMesh.GetBoundingBox` (`self.Static Mesh`))))
  (bind _returnvalue_x (`KismetMathLibrary.BreakVector` (+ (`KismetMathLibrary.Vector_GetAbs` _returnvalue_min) (`KismetMathLibrary.Vector_GetAbs` _returnvalue_max))))
  ;[1 1 1 0.5] Spline mesh measuring tool
  ;;[1 1 1] Updates the text with the length of the spline
  (`parent.UserConstructionScript`)
  (`TextRenderComponent.K2_SetText` (`self.Text`) (`KismetTextLibrary.Conv_DoubleToText` (`SplineComponent.GetSplineLength` (`self.Spline`)) "HalfToEven"))
  (`StaticMeshComponent.SetStaticMesh` (`self.InstancedStaticMesh`) (`self.Static Mesh`))
  (`InstancedStaticMeshComponent.ClearInstances` (`self.InstancedStaticMesh`))
  ;;[1 1 1] Find the length of the static mesh
  (set `self.XLength` (* _returnvalue_x (`self.Static Mesh Size Multiplier`)))
  (for _index (range (+ (`KismetMathLibrary.FTrunc` (/ (`SplineComponent.GetSplineLength` (`self.Spline`)) (`self.XLength`))) 1))
    ;;[1 1 1] Spawn static mesh at location along spline
    (`InstancedStaticMeshComponent.AddInstance` (`self.InstancedStaticMesh`) (`KismetMathLibrary.MakeTransform` (`SplineComponent.GetLocationAtDistanceAlongSpline` (`self.Spline`) (+ (* _index (`self.XLength`)) (/ (`self.XLength`) 2.0)) "Local") (struct) (`KismetMathLibrary.MakeVector` _static_mesh_size_multiplier _static_mesh_size_multiplier _static_mesh_size_multiplier)) false))
  ;;[1 1 1] Set the material of the static mesh
  (`PrimitiveComponent.SetMaterial` (`self.InstancedStaticMesh`) 0 (`self.Main Color`)))