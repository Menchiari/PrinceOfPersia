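; BP_CoverTool is a level design toolkit actor that draws a cover-sized box labeled with its dimensions.
; The construction script scales and centers a cube from the Corner vector, so it spans from the actor origin to that point, and applies MainColor.
; X, Y and Z text components show each size at the midpoint of its axis, with Y shown as an absolute value.
; It has no active runtime logic.
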(fn `UserConstructionScript`
  (bind _corner_x (`KismetMathLibrary.BreakVector` (`self.Corner`)))
  (bind (_corner_x_2 _corner_y) (`KismetMathLibrary.BreakVector` (`self.Corner`)))
  (bind (_corner_x_3 _corner_y_2 _corner_z) (`KismetMathLibrary.BreakVector` (`self.Corner`)))
  (`parent.UserConstructionScript`)
  ;[1 1 1] Set scale of the box
  (`SceneComponent.SetWorldScale3D` (`self.Cube`) (/ (`self.Corner`) 100))
  ;[1 1 1] Set the position of the box
  (`SceneComponent.K2_SetRelativeLocation` (`self.Cube`) (/ (`self.Corner`) 2) false false)
  ;[1 1 1] Set the material of the box
  (`PrimitiveComponent.SetMaterial` (`self.Cube`) 0 (`self.Main Color`))
  ;[1 1 1] Set the X size text and position
  (`TextRenderComponent.K2_SetText` (`self.X`) (`KismetTextLibrary.Conv_DoubleToText` _corner_x "HalfToEven"))
  (`SceneComponent.K2_SetRelativeLocation` (`self.X`) (`KismetMathLibrary.MakeVector` (/ _corner_x 2.0) -1.0) false false)
  ;[1 1 1] Set the Y size text and position
  (`TextRenderComponent.K2_SetText` (`self.Y`) (`KismetTextLibrary.Conv_DoubleToText` (`KismetMathLibrary.Abs` _corner_y) "HalfToEven"))
  (`SceneComponent.K2_SetRelativeLocation` (`self.Y`) (`KismetMathLibrary.MakeVector` -1.0 (/ _corner_y 2.0)) false false)
  ;[1 1 1] Set the Z size text and position
  (`TextRenderComponent.K2_SetText` (`self.Z`) (`KismetTextLibrary.Conv_DoubleToText` _corner_z "HalfToEven"))
  (`SceneComponent.K2_SetRelativeLocation` (`self.Z`) (`KismetMathLibrary.MakeVector` -1.0 0.0 (/ _corner_z 2.0)) false false))