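; Player character Blueprint that adds an Enhanced Input mapping context and relays movement input to its animation Blueprint.
; Left, Right and Shift start and completion events write their values into ABP_Character.
; Only held Right moves the character, through a Movement event that offsets the capsule along world X, then re-calls itself after a delay with zero speed.
; Up and Down inputs are empty stubs.
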(event `self.ReceiveBeginPlay`
  (bind _asplayer_controller (cast `PlayerController` (`self.GetController`)))
  (bind _returnvalue (pcsubsystem `EnhancedInputLocalPlayerSubsystem` _asplayer_controller))
  (`/Engine/EditorBlueprintResources/StandardMacros.IsValid` _returnvalue
    (:`Is Valid`
      (`EnhancedInputSubsystemInterface.AddMappingContext` _returnvalue "/Game/Blueprints/IM_Character_Player.IM_Character_Player" 0 (struct)))))

(event `EnhancedInput|/Game/InputAction_Left`
  (params (ActionValue :type Boolean) (ElapsedSeconds :type "Float (double-precision)") (TriggeredSeconds :type "Float (double-precision)") (InputAction :type "InputAction Object Reference" :default "/Game/InputAction_Left.InputAction_Left"))
  (:`Started`
    (bind _asabp_character (cast `/Game/Blueprints/ABP_Character` (`SkeletalMeshComponent.GetAnimInstance` (`self.Mesh`)) :!label _label))
    (set `/Game/Blueprints/ABP_Character.Left` ActionValue _asabp_character))
  (:`Completed`
    (goto _label)))

(event `Movement`
  (params (Speed :type "Float (double-precision)"))
  (bind _capsulecomponent (`self.CapsuleComponent`))
  (bind (_returnvalue_x _returnvalue_y _returnvalue_z) (`KismetMathLibrary.BreakVector` (`SceneComponent.K2_GetComponentLocation` _capsulecomponent)))
  (if true
    (`SceneComponent.K2_SetWorldLocation` _capsulecomponent (`KismetMathLibrary.MakeVector` (+ Speed _returnvalue_x) _returnvalue_y _returnvalue_z) false false)
    (`KismetSystemLibrary.Delay` 0.1)
    (`self.Movement` 0.0)))

(event `EnhancedInput|/Game/InputAction_Right`
  (params (ActionValue :type Boolean) (ElapsedSeconds :type "Float (double-precision)") (TriggeredSeconds :type "Float (double-precision)") (InputAction :type "InputAction Object Reference" :default "/Game/InputAction_Right.InputAction_Right"))
  (:`Triggered`
    (`self.Movement` 1.0))
  (:`Started`
    (bind _asabp_character (cast `/Game/Blueprints/ABP_Character` (`SkeletalMeshComponent.GetAnimInstance` (`self.Mesh`)) :!label _label_2))
    (set `/Game/Blueprints/ABP_Character.Right` ActionValue _asabp_character))
  (:`Completed`
    (goto _label_2)))

(event `EnhancedInput|/Game/InputAction_Shift`
  (params (ActionValue :type Boolean) (ElapsedSeconds :type "Float (double-precision)") (TriggeredSeconds :type "Float (double-precision)") (InputAction :type "InputAction Object Reference" :default "/Game/InputAction_Shift.InputAction_Shift"))
  (:`Started`
    (bind _asabp_character (cast `/Game/Blueprints/ABP_Character` (`SkeletalMeshComponent.GetAnimInstance` (`self.Mesh`)) :!label _label_3))
    (set `/Game/Blueprints/ABP_Character.Shift` ActionValue _asabp_character))
  (:`Completed`
    (goto _label_3)))

(event `EnhancedInput|/Game/InputAction_Down`
  (params (ActionValue :type Boolean) (ElapsedSeconds :type "Float (double-precision)") (TriggeredSeconds :type "Float (double-precision)") (InputAction :type "InputAction Object Reference" :default "/Game/InputAction_Down.InputAction_Down")))

(event `EnhancedInput|/Game/InputAction_Up`
  (params (ActionValue :type Boolean) (ElapsedSeconds :type "Float (double-precision)") (TriggeredSeconds :type "Float (double-precision)") (InputAction :type "InputAction Object Reference" :default "/Game/InputAction_Up.InputAction_Up")))

(fn `UserConstructionScript`)